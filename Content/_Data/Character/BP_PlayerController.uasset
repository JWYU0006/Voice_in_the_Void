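; Player controller for point-and-click play, handling movement, interaction, dialogue clicks and the main HUD.
; Holding left mouse navigates the pawn toward the cursor hit, while Tick blends walk speed by distance to that point.
; Highlighted targets trigger on click or arrival within range, with actor tags selecting circuit breaker, locker keypad or door removal.
; Mode flags gate movement and route clicks, and the game instance logs input events.
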(event `self.ReceiveTick`
  (params (DeltaSeconds :type "Float (single-precision)"))
  (bind _returnvalue (`GameplayStatics.GetPlayerPawn` 0))
  (bind _returnvalue_2 (`GameplayStatics.GetWorldDeltaSeconds`))
  (bind _returnvalue_3 (`KismetMathLibrary.Vector_Distance` (`self.Hit Result Location`) (`self.K2_GetActorLocation` _returnvalue)))
  ; Check character arrived for interaction and signifier invisible logic and movement logic
  (if (`self.IsHeld`)
    (`self.MovementLogic`))
  (`self.GoInvisible`)
  (bind _asbp_player_character (cast `/Game/_Data/Character/BP_PlayerCharacter` _returnvalue))
  (`|ExecutionSequence`
    (:`then_0`
      (if (`KismetSystemLibrary.IsValid` (`self.InteractableTarget`))
        (if (< (`KismetMathLibrary.Vector_Distance` (`self.K2_GetActorLocation` (`self.InteractableTarget`)) (`self.K2_GetActorLocation` (`GameplayStatics.GetPlayerPawn` 0))) 200.0)
          (if (`self.ToTarget`)
            (`KismetSystemLibrary.PrintString` "Interacted")
            (set `self.ToTarget` false)
            (`self.OpenMinigame`)
            (elif (not (`self.Highlighted`))
              (set `self.InteractableTarget` null))))))
    (:`then_1`
      (if (>= _returnvalue_3 300.0)
        (bind _charactermovement (`Character.CharacterMovement` _asbp_player_character))
        (bind _returnvalue_4 (`MovementComponent.GetMaxSpeed` _charactermovement))
        (set `CharacterMovementComponent.MaxWalkSpeed` (`KismetMathLibrary.FInterpTo` _returnvalue_4 (`self.RunSpeed`) _returnvalue_2 2.5) _charactermovement)
        (elif (>= _returnvalue_3 170.0)
          (set `CharacterMovementComponent.MaxWalkSpeed` (`KismetMathLibrary.FInterpTo` _returnvalue_4 (`self.FastWalkSpeed`) _returnvalue_2 2.5) _charactermovement)
          (else
            (set `CharacterMovementComponent.MaxWalkSpeed` (`KismetMathLibrary.FInterpTo` _returnvalue_4 (`self.WalkSpeed`) _returnvalue_2 2.5) _charactermovement)))))))

(event `self.ReceiveBeginPlay`
  ; Initiate and add UI
  (bind _returnvalue (`|CreateWidget` "/Game/_Data/UI/WBP_MainHUD.WBP_MainHUD_C"))
  (bind _output_get (set `self.WBPMainHUD` _returnvalue))
  (`UserWidget.AddToViewport` _output_get 0))

(event `Key|AnyKey`
  (params (Key :type "Key Structure"))
  (:`Pressed`
    (bind _asgi_voice_in_the_void (cast `/Game/_Data/Blueprints/GI_VoiceInTheVoid` (`GameplayStatics.GetGameInstance`)))
    (`/Game/_Data/Blueprints/GI_VoiceInTheVoid.LogPasscodeData` _asgi_voice_in_the_void "Key Pressed" (0.0 0.0) Key)))

(event `Key|LeftMouseButton`
  (params (Key :type "Key Structure"))
  ; Mouse input if held down or not
  (:`Pressed`
    (set `self.IsHeld` true))
  (:`Released`
    (set `self.IsHeld` false)))

(event `Key|Escape`
  (params (Key :type "Key Structure"))
  (:`Pressed`
    (`KismetSystemLibrary.QuitGame` null "Quit")))

(event `Key|LeftMouseButton`
  (params (Key :type "Key Structure"))
  (bind (_locationx _locationy) (`self.GetMousePosition`))
  (bind _wbpmainhud (`self.WBPMainHUD`))
  (bind _returnvalue (`KismetStringLibrary.Conv_StringToInt` (`KismetStringLibrary.Conv_NameToString` (`self.Index`))))
  ; Mouse interaction for UI dialogue
  (:`Pressed`
    (if (`self.IsDialogue`)
      (bind _asgi_voice_in_the_void (cast `/Game/_Data/Blueprints/GI_VoiceInTheVoid` (`GameplayStatics.GetGameInstance`)))
      (`/Game/_Data/Blueprints/GI_VoiceInTheVoid.LogDialogueData` _asgi_voice_in_the_void "" (`KismetMathLibrary.MakeVector2D` _locationx _locationy))
      (bind _asbp_dialogue_collision (cast `/Game/_Data/Blueprints/BP_DialogueCollision` (`self.CurrentDialogueActor`)))
      (for _array_element (`/Game/_Data/Blueprints/BP_DialogueCollision.Options` _asbp_dialogue_collision)
        _)
      (bind (_section _startn _endn _conditions _gameplaytagadded _gameplaytagremoved _customlist _namelistcustomlistenabled) (break `/Game/_Data/Blueprints/S_DialogueOptions` _array_element))
      (if _customlist
        (set `self.Index` (`KismetStringLibrary.Conv_StringToName` (`KismetStringLibrary.Conv_IntToString` (+ _returnvalue 1))))
        (if (`KismetArrayLibrary.Array_IsValidIndex` _namelistcustomlistenabled _returnvalue)
          (`/Game/_Data/UI/Dialogue/WBP_Dialogue.UpdateDialogue` (`/Game/_Data/UI/WBP_MainHUD.WBP_Dialogue` (`self.WBPMainHUD`)) (`|GetArrayItem` _namelistcustomlistenabled _returnvalue) 0 "None" true)
          (else
            (`Widget.SetVisibility` (`/Game/_Data/UI/WBP_MainHUD.WBP_Dialogue` _wbpmainhud) "Hidden")
            (`Widget.SetVisibility` (`/Game/_Data/UI/WBP_MainHUD.WBP_Character` _wbpmainhud) "Hidden")
            (`Widget.SetVisibility` (`/Game/_Data/UI/WBP_MainHUD.WBP_Character_1` _wbpmainhud) "Hidden")
            (`Widget.SetVisibility` (`/Game/_Data/UI/WBP_MainHUD.WBP_Name` _wbpmainhud) "Hidden")
            (`Widget.SetVisibility` (`/Game/_Data/UI/WBP_MainHUD.WBP_Name_1` _wbpmainhud) "Hidden")
            (set `self.IsDialogue` false)))
        (else
          (bind _output_get (set `self.Index` (`KismetStringLibrary.Conv_StringToName` (`KismetStringLibrary.Conv_IntToString` (+ (`KismetStringLibrary.Conv_StringToInt` (`KismetStringLibrary.Conv_NameToString` (`self.Index`))) 1)))))
          (`/Game/_Data/UI/Dialogue/WBP_Dialogue.UpdateDialogue` (`/Game/_Data/UI/WBP_MainHUD.WBP_Dialogue` (`self.WBPMainHUD`)) _output_get _section _endn false)))
      (else
        (`Widget.SetVisibility` (`/Game/_Data/UI/WBP_MainHUD.WBP_Dialogue` (`self.WBPMainHUD`)) "Hidden")))))

(event `Key|LeftMouseButton`
  (params (Key :type "Key Structure"))
  (bind (_locationx _locationy) (`self.GetMousePosition`))
  ; Check if character is already within range of interaction
  (:`Pressed`
    (if (`self.IsPasscode`)
      (bind _asgi_voice_in_the_void (cast `/Game/_Data/Blueprints/GI_VoiceInTheVoid` (`GameplayStatics.GetGameInstance`)))
      (`/Game/_Data/Blueprints/GI_VoiceInTheVoid.LogPasscodeData` _asgi_voice_in_the_void "Left Mouse Click" (`KismetMathLibrary.MakeVector2D` _locationx _locationy) "None")
      (elif (`self.IsDialogue`)
        _
        (elif (`self.IsClimbing`)
          _
          (elif (`self.Highlighted`)
            (if (`KismetSystemLibrary.IsValid` (`self.InteractableTarget`))
              (if (< (`KismetMathLibrary.Vector_Distance` (`self.K2_GetActorLocation` (`self.InteractableTarget`)) (`self.K2_GetActorLocation` (`GameplayStatics.GetPlayerPawn` 0))) 200.0)
                (`KismetSystemLibrary.PrintString` "Interacted")
                (`self.OpenMinigame`)
                (else
                  (set `self.ToTarget` true)
                  (`KismetSystemLibrary.PrintString` "Going to target")))
              (else
                (`KismetSystemLibrary.PrintString` "Not found" :!label _label)
                (set `self.ToTarget` false)))
            (else
              (set `self.InteractableTarget` null)
              (goto _label))))))))

(fn `MovementLogic`
  (bind (_hitresult _returnvalue) (`self.GetHitResultUnderCursorByChannel` "TraceTypeQuery3"))
  (if (`self.IsCircuitBreaker`)
    _
    (elif (`self.IsPasscode`)
      _
      (elif (`self.IsDialogue`)
        _
        (elif (`self.IsClimbing`)
          (`KismetSystemLibrary.PrintString` "climbing")
          (else
            (bind _output_get (set `self.Hit Result Location` (`.Location` (`GameplayStatics.BreakHitResult` _hitresult))))
            (if (not (== (`KismetMathLibrary.Vector_Zero`) _output_get))
              (bind _asgi_voice_in_the_void (cast `/Game/_Data/Blueprints/GI_VoiceInTheVoid` (`GameplayStatics.GetGameInstance`)))
              (if (`self.IsHeld`)
                (`AIBlueprintHelperLibrary.SimpleMoveToLocation` self (`.Location` (`GameplayStatics.BreakHitResult` _hitresult)) :!label _label)
                (`self.MouseClicked`)
                (`self.K2_SetActorRotation` (`self.K2_GetPawn`) (`KismetMathLibrary.RInterpTo` (`self.K2_GetActorRotation` (`self.K2_GetPawn`)) (`KismetMathLibrary.FindLookAtRotation` (`self.K2_GetActorLocation` (`self.K2_GetPawn`)) (`.Location` (`GameplayStatics.BreakHitResult` _hitresult))) 0.0 1.0) false)
                (set `self.IsScanner` false)
                (else
                  (`/Game/_Data/Blueprints/GI_VoiceInTheVoid.LogNavData` _asgi_voice_in_the_void "Left Mouse Click" _output_get (`self.InteractableTarget`))
                  (if _returnvalue
                    (goto _label)))))))))))

(fn `OpenCircuitBreaker`
  (`Widget.SetVisibility` (`/Game/_Data/UI/WBP_MainHUD.WBP_CircuitBreaker` (`self.WBPMainHUD`)) "Visible")
  (set `self.IsCircuitBreaker` true))

(fn `OpenCodePad`
  (bind _foundwidgets (`WidgetBlueprintLibrary.GetAllWidgetsOfClass` "/Game/_Data/UI/Passcode/WBP_CodePad.WBP_CodePad_C"))
  (for _array_element _foundwidgets
    (`Widget.RemoveFromParent` _array_element))
  (bind _asbp_locker (cast `/Game/_Data/Blueprints/BP_Locker` (`self.InteractableTarget`)))
  (bind _returnvalue (`|CreateWidget` "/Game/_Data/UI/Passcode/WBP_Passcode.WBP_Passcode_C" (`GameplayStatics.GetPlayerController` 0)))
  (set `/Game/_Data/UI/Passcode/WBP_CodePad.Password` (`/Game/_Data/Blueprints/BP_Locker.Password` _asbp_locker) (`/Game/_Data/UI/Passcode/WBP_Passcode.WBP_CodePad` _returnvalue))
  (`UserWidget.AddToViewport` _returnvalue 0)
  (set `self.SelectedLocker` (`self.InteractableTarget`))
  (set `self.IsPasscode` true))

(fn `OpenMinigame`
  (if (`self.ActorHasTag` (`self.InteractableTarget`) "CircuitBreaker")
    (`self.OpenCircuitBreaker`)
    (elif (`self.ActorHasTag` (`self.InteractableTarget`) "Passcode")
      (`self.OpenCodePad`)
      (elif (`self.ActorHasTag` (`self.InteractableTarget`) "Door")
        (if (`self.ActorHasTag` (`self.InteractableTarget`) "Openable")
          (`self.K2_DestroyActor` (`self.InteractableTarget`)))))))

(fn `UserConstructionScript`)
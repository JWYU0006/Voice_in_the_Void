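; BP_PlayerCharacter is the player character Blueprint, which seeds a set of tags and attaches clothing animation to the body.
; On BeginPlay it adds tags to its BPCTagManager component: a StateTree test tag, a scanner flag and several dialogue-playable flags.
; The construction script sets Mesh as the leader pose component of Clothes2, so the clothing follows the body's animation.
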(event `self.ReceiveBeginPlay`
  (`/Game/_Data/Blueprints/BPC_TagManager.AddTag` (`self.BPC_TagManager`) (struct :`TagName` "Test.StateTree.Tag"))
  (`/Game/_Data/Blueprints/BPC_TagManager.AddTag` (`self.BPC_TagManager`) (struct :`TagName` "HasScanner"))
  (`/Game/_Data/Blueprints/BPC_TagManager.AddTag` (`self.BPC_TagManager`) (struct :`TagName` "IsDialoguePlayable"))
  (`/Game/_Data/Blueprints/BPC_TagManager.AddTag` (`self.BPC_TagManager`) (struct :`TagName` "IsDialoguePlayable2"))
  (`/Game/_Data/Blueprints/BPC_TagManager.AddTag` (`self.BPC_TagManager`) (struct :`TagName` "IsDialoguePlayable3"))
  (`/Game/_Data/Blueprints/BPC_TagManager.AddTag` (`self.BPC_TagManager`) (struct :`TagName` "IsDialoguePlayable4"))
  (`/Game/_Data/Blueprints/BPC_TagManager.AddTag` (`self.BPC_TagManager`) (struct :`TagName` "IsDialoguePlayable5")))

(event `self.ReceiveTick`
  (params (DeltaSeconds :type "Float (single-precision)")))

(fn `UserConstructionScript`
  (`SkinnedMeshComponent.SetLeaderPoseComponent` (`self.Clothes-2`) (`self.Mesh`) false false))
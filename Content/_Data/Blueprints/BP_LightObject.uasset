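; BP_LightObject is a Blueprint light that can be switched on and off through events.
; On BeginPlay it caches the point light's starting intensity and binds its handlers to the TurnLightOn and TurnLightOff events.
; Turning off sets intensity to zero, turning on restores the cached value, and each prints a debug message.
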(event `self.ReceiveBeginPlay`
  (set `self.OldIntensity` (`LightComponentBase.Intensity` (`self.PointLight`)))
  (add `self.TurnLightOn` (delegate `LightOn`))
  (add `self.TurnLightOff` (delegate `LightOff`)))

(event `LightOn`
  (`KismetSystemLibrary.PrintString` "Light Turned On")
  (`LightComponent.SetIntensity` (`self.PointLight`) (`self.OldIntensity`)))

(event `LightOff`
  (`KismetSystemLibrary.PrintString` "Light Turned Off")
  (`LightComponent.SetIntensity` (`self.PointLight`) 0.0))

(fn `UserConstructionScript`)
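; BP_DialogueCollision is an overlap-triggered actor that starts tag-conditioned dialogue in the main HUD.
; On overlap it registers itself with the player controller and bubble-sorts its Options by condition count, most first.
; Every option matching the player's tags, checked in turn without stopping at the first, edits those tags and updates the dialogue widget from a custom list or section range.
; Matches also show character widgets with hardcoded speaker names.
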(event `self.ReceiveActorBeginOverlap`
  (params (OtherActor :type "Actor Object Reference"))
  ; Initiate variables
  (bind _asbp_player_controller (cast `/Game/_Data/Character/BP_PlayerController` (`GameplayStatics.GetPlayerController` 0)))
  (set `/Game/_Data/Character/BP_PlayerController.CurrentDialogueActor` self _asbp_player_controller)
  ; Sort and check conditions
  (`self.SortGameplayTag`)
  (for _array_element (`self.Options`)
    (bind _asbp_player_character (cast `/Game/_Data/Character/BP_PlayerCharacter` (`GameplayStatics.GetPlayerPawn` 0)))
    (bind _bpc_tagmanager (`/Game/_Data/Character/BP_PlayerCharacter.BPC_TagManager` _asbp_player_character))
    (bind (_section _startn _endn _conditions _gameplaytagadded _gameplaytagremoved _customlist _namelistcustomlistenabled) (break `/Game/_Data/Blueprints/S_DialogueOptions` _array_element))
    (if (`BlueprintGameplayTagLibrary.HasAllTags` (`/Game/_Data/Blueprints/BPC_TagManager.GameplayTags` _bpc_tagmanager) _conditions true)
      (for _array_element_2 (`BlueprintGameplayTagLibrary.BreakGameplayTagContainer` _gameplaytagadded)
        (`/Game/_Data/Blueprints/BPC_TagManager.AddTag` _bpc_tagmanager _array_element_2))
      (for _array_element_3 (`BlueprintGameplayTagLibrary.BreakGameplayTagContainer` _gameplaytagremoved)
        (`/Game/_Data/Blueprints/BPC_TagManager.RemoveTag` _bpc_tagmanager _array_element_3))
      ; Initiate dialogue system
      (bind _asbp_player_controller_2 (cast `/Game/_Data/Character/BP_PlayerController` (`GameplayStatics.GetPlayerController` 0)))
      (if _customlist
        (bind _output_get (set `/Game/_Data/Character/BP_PlayerController.Index` "0" _asbp_player_controller_2))
        (`KismetSystemLibrary.PrintString` (`KismetStringLibrary.Conv_NameToString` _output_get))
        (bind _wbp_dialogue (`/Game/_Data/UI/WBP_MainHUD.WBP_Dialogue` (`/Game/_Data/Character/BP_PlayerController.WBPMainHUD` _asbp_player_controller)))
        (`/Game/_Data/UI/Dialogue/WBP_Dialogue.UpdateDialogue` _wbp_dialogue (`|GetArrayItem` _namelistcustomlistenabled) 0 "None" true)
        (else
          (bind _output_get_2 (set `/Game/_Data/Character/BP_PlayerController.Index` _startn _asbp_player_controller_2))
          (`/Game/_Data/UI/Dialogue/WBP_Dialogue.UpdateDialogue` _wbp_dialogue _output_get_2 _section _endn false)))
      (bind _wbpmainhud (`/Game/_Data/Character/BP_PlayerController.WBPMainHUD` _asbp_player_controller_2))
      (`Widget.SetVisibility` (`/Game/_Data/UI/WBP_MainHUD.WBP_Dialogue` _wbpmainhud) "Visible")
      (`Widget.SetVisibility` (`/Game/_Data/UI/WBP_MainHUD.WBP_Character` _wbpmainhud) "Visible")
      (`Widget.SetVisibility` (`/Game/_Data/UI/WBP_MainHUD.WBP_Character_1` _wbpmainhud) "Visible")
      (`TextBlock.SetText` (`/Game/_Data/UI/Dialogue/WBP_Name.NameText` (`/Game/_Data/UI/WBP_MainHUD.WBP_Name` _wbpmainhud)) "Scientist")
      (`TextBlock.SetText` (`/Game/_Data/UI/Dialogue/WBP_Name.NameText` (`/Game/_Data/UI/WBP_MainHUD.WBP_Name_1` _wbpmainhud)) "Unknown")
      (else
        (`KismetSystemLibrary.PrintString` "Tags do not match")))))

(fn `SortGameplayTag`
  (locals (TempGameplayTag :type "GameplayTagContainer Structure"))
  (bind _options (`self.Options`))
  ; Outer loop
  (for _ (range (`KismetArrayLibrary.Array_Length` (`self.Options`)))
    ; Inner Loop
    (for _index (range (+ (- (`KismetArrayLibrary.Array_Length` (`self.Options`)) 2) 1))
      (bind (_output_section _output_startn _output_endn _output_conditions) (break `/Game/_Data/Blueprints/S_DialogueOptions` (`|GetArrayItem` _options _index)))
      (bind _returnvalue (+ _index 1))
      (bind (_output_section_2 _output_startn_2 _output_endn_2 _output_conditions_2) (break `/Game/_Data/Blueprints/S_DialogueOptions` (`|GetArrayItem` _options _returnvalue)))
      ; Swap the index if is smaller
      (if (< (`BlueprintGameplayTagLibrary.GetNumGameplayTagsInContainer` _output_conditions) (`BlueprintGameplayTagLibrary.GetNumGameplayTagsInContainer` _output_conditions_2))
        (`KismetArrayLibrary.Array_Swap` (`self.Options`) _index _returnvalue)
        (`KismetSystemLibrary.PrintString` "Swapped")
        (else
          (`KismetSystemLibrary.PrintString` "Not Swapped"))))))

(fn `UserConstructionScript`)
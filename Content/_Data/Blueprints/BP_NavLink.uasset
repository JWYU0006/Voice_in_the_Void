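; BP_NavLink is a smart nav link that animates the player climbing up or down ledges or ladders.
; On reach, it traces down to find the landing surface, stops the player controller and flags it as climbing.
; Timelines lerp the player pawn vertically then forward when ascending, or forward then vertically when descending, offset by capsule half-height.
; Afterwards it clears the flag and restores Walking; the node setting movement mode None is unconnected.
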(event `self.ReceiveSmartLinkReached`
  (params (Agent :type "Actor Object Reference") (Destination :type "Vector Structure (by ref)"))
  (bind (_destination_x _destination_y _destination_z) (`KismetMathLibrary.BreakVector` (`self.Destination`)))
  (bind (_destination_x_2 _destination_y_2 _destination_z_2) (`KismetMathLibrary.BreakVector` (`self.Destination`)))
  (bind (_destination_x_3 _destination_y_3) (`KismetMathLibrary.BreakVector` (`self.Destination`)))
  (bind (_destination_x_4 _destination_y_4 _destination_z_3) (`KismetMathLibrary.BreakVector` (`self.Destination`)))
  (bind (_lerpstart_x _lerpstart_y) (`KismetMathLibrary.BreakVector` (`self.LerpStart`)))
  (bind (_destination_x_5 _destination_y_5 _destination_z_4) (`KismetMathLibrary.BreakVector` (`self.Destination`)))
  (bind (_lerpstart_x_2 _lerpstart_y_2) (`KismetMathLibrary.BreakVector` (`self.LerpStart`)))
  (bind (_destination_x_6 _destination_y_6 _destination_z_5) (`KismetMathLibrary.BreakVector` (`self.Destination`)))
  (bind (_lerpstart_x_3 _lerpstart_y_3 _lerpstart_z) (`KismetMathLibrary.BreakVector` (`self.LerpStart`)))
  (bind (_returnvalue_x _returnvalue_y _returnvalue_z) (`KismetMathLibrary.BreakVector` (`self.K2_GetActorLocation` (`self.Agent`))))
  (bind _returnvalue (`KismetMathLibrary.MakeVector` _lerpstart_x_2 _lerpstart_y_2 (+ _destination_z_4 (`CapsuleComponent.CapsuleHalfHeight` (`self.As Capsule Collision`)))))
  ; Initiate variables
  (set `self.Agent` Agent)
  (bind _output_get (set `self.Destination` Destination))
  (bind _outhit (`KismetSystemLibrary.LineTraceSingle` _output_get (`KismetMathLibrary.MakeVector` _destination_x_2 _destination_y_2 (- _destination_z_2 10000.0)) "TraceTypeQuery1"))
  (set `self.Destination` (`.Location` (`GameplayStatics.BreakHitResult` _outhit)))
  (bind _ascapsule_collision (cast `CapsuleComponent` (`Actor.RootComponent` (`GameplayStatics.GetPlayerPawn` 0))))
  (set `self.As Capsule Collision` _ascapsule_collision)
  ; Stop movement to prepare for climb
  (bind _asbp_player_controller (cast `/Game/_Data/Character/BP_PlayerController` (`GameplayStatics.GetPlayerController` 0)))
  (set `self.As BP Player Controller` _asbp_player_controller)
  (set `/Game/_Data/Character/BP_PlayerController.IsClimbing` true (`self.As BP Player Controller`))
  (`Controller.StopMovement` (`self.As BP Player Controller`))
  (bind _asbp_player_character (cast `/Game/_Data/Character/BP_PlayerCharacter` (`self.Agent`)))
  (if (> _destination_z_3 _returnvalue_z)
    ; Vertical Lerp
    (set `self.LerpStart` (`self.K2_GetActorLocation` (`self.Agent`)))
    (bind (_direction _alpha) (`Timeline|LadderClimbCurve` :!via `PlayFromStart`)
      (:`Update`
        (`self.K2_SetActorLocation` (`GameplayStatics.GetPlayerPawn` 0) (`KismetMathLibrary.VLerp` (`self.LerpStart`) _returnvalue _alpha) false false))
      (:`Finished`
        ; Horizontal Lerp
        (bind (_direction_2 _alpha_2) (`Timeline|ForwardCurve` :!via `PlayFromStart`)
          (:`Update`
            (`self.K2_SetActorLocation` (`GameplayStatics.GetPlayerPawn` 0) (`KismetMathLibrary.VLerp` _returnvalue (`KismetMathLibrary.MakeVector` _destination_x_6 _destination_y_6 (+ _destination_z_5 (`CapsuleComponent.CapsuleHalfHeight` (`self.As Capsule Collision`)))) _alpha_2) false false))
          (:`Finished`
            ; Change movement mode back once climbing is finished
            (set `/Game/_Data/Character/BP_PlayerController.IsClimbing` false (`self.As BP Player Controller`) :!label _label)
            (bind _asbp_player_character_2 (cast `/Game/_Data/Character/BP_PlayerCharacter` (`self.Agent`)))
            (`CharacterMovementComponent.SetMovementMode` (`Character.CharacterMovement` _asbp_player_character_2) "MOVE_Walking" 0)))))
    (else
      ; Horizontal Lerp
      (set `self.LerpStart` (`self.K2_GetActorLocation` (`self.Agent`)))
      (bind (_direction_3 _alpha_3) (`Timeline|Timeline_0` :!via `PlayFromStart`)
        (:`Update`
          (`self.K2_SetActorLocation` (`GameplayStatics.GetPlayerPawn` 0) (`KismetMathLibrary.VLerp` (`KismetMathLibrary.MakeVector` _lerpstart_x_3 _lerpstart_y_3 _lerpstart_z) (`KismetMathLibrary.MakeVector` _destination_x_3 _destination_y_3 _lerpstart_z) _alpha_3) false false))
        (:`Finished`
          ; Vertical Lerp
          (set `self.LerpStart` (`self.K2_GetActorLocation` (`self.Agent`)))
          (bind (_direction_4 _alpha_4) (`Timeline|Timeline` :!via `PlayFromStart`)
            (:`Update`
              (`self.K2_SetActorLocation` (`GameplayStatics.GetPlayerPawn` 0) (`KismetMathLibrary.VLerp` (`self.LerpStart`) (`KismetMathLibrary.MakeVector` _lerpstart_x _lerpstart_y (+ _destination_z (`CapsuleComponent.CapsuleHalfHeight` (`self.As Capsule Collision`)))) _alpha_4) false false))
            (:`Finished`
              (goto _label))))))))

(fn `UserConstructionScript`)
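; Game instance for Voice in the Void that owns the telemetry service used to record player behaviour.
; On Init it creates and connects the service, then on a successful connection logs the entered level and caches the player controller.
; Helper functions log power grid, scanner, navigation, dialogue and passcode interactions as JSON events tagged by section.
; Each helper sends only if the connection succeeded.
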(event `self.ReceiveInit`
  (bind _returnvalue (`|GenericCreateObject` "/Game/Telemetry/TelemetryService.TelemetryService_C" "https://dd-telemetry-odd-e1dd6794cd3d.herokuapp.com/" "Red Cat" "threshold straw"))
  (bind _output_get (set `self.TelemetryService` _returnvalue))
  (add `/Game/Telemetry/TelemetryService.On Connection Result` _output_get (delegate `OnTelemetryConnectionResult`))
  (`/Game/Telemetry/TelemetryService.Try Connect` _output_get))

(event `OnTelemetryConnectionResult`
  (params (Success :type Boolean) (`Session Index` :type Integer) (Message :type String))
  (bind _output_get (set `self.Success` Success))
  (set `self.Session` (`KismetTextLibrary.Conv_IntToText` `Session Index`))
  (if _output_get
    (`/Game/Telemetry/TelemetryService.Set Section` (`self.TelemetryService`) "Roaming")
    (bind _structout (setmembers `JsonObjectWrapper` :`StructRef` (make `JsonObjectWrapper`)))
    (bind _returnvalue (`GameplayStatics.GetCurrentLevelName` true))
    (`|SetJsonField` _structout "Scene ID" _returnvalue)
    (`/Game/Telemetry/TelemetryService.Log Event` (`self.TelemetryService`) "Entered Scene" "" _structout)
    (bind _asbp_player_controller (cast `/Game/_Data/Character/BP_PlayerController` (`GameplayStatics.GetPlayerController` 0)))
    (set `self.As BP Player Controller` _asbp_player_controller)))

(fn `LogDialogueData`
  (params (`Event Name` :type String) (`Mouse Screen Position` :type "Vector2D Structure"))
  (bind _jsonobjectwrapper (make `JsonObjectWrapper`))
  (bind _jsonobjectwrapper_2 (make `JsonObjectWrapper`))
  (bind _jsonobjectwrapper_3 (make `JsonObjectWrapper`))
  (if (`self.Success`)
    (`|SetJsonField` _jsonobjectwrapper_3 "Event ID" `Event Name`)
    (`|SetJsonField` _jsonobjectwrapper_2 "Mouse Screen Position" `Mouse Screen Position`)
    (`|SetJsonField` _jsonobjectwrapper "Data" (`|MakeArray` _jsonobjectwrapper_3 _jsonobjectwrapper_2))
    (`/Game/Telemetry/TelemetryService.Set Section` (`self.TelemetryService`) "Dialogue")
    (`/Game/Telemetry/TelemetryService.Log Event` (`self.TelemetryService`) "DialogueUI" "" _jsonobjectwrapper)))

(fn `LogNavData`
  (params (`Event Name` :type String) (`Mouse World Position` :type "Vector Structure") (Target :type "Actor Object Reference"))
  (bind _jsonobjectwrapper (make `JsonObjectWrapper`))
  (bind _jsonobjectwrapper_2 (make `JsonObjectWrapper`))
  (bind _jsonobjectwrapper_3 (make `JsonObjectWrapper`))
  (bind _jsonobjectwrapper_4 (make `JsonObjectWrapper`))
  (bind _jsonobjectwrapper_5 (make `JsonObjectWrapper`))
  (if (`self.Success`)
    (`|SetJsonField` _jsonobjectwrapper_4 "Event ID" `Event Name`)
    (`|SetJsonField` _jsonobjectwrapper_3 "Mouse World Position" `Mouse World Position`)
    (`|SetJsonField` _jsonobjectwrapper_5 "Interact Target Name" (`KismetSystemLibrary.GetObjectName` Target))
    (`|SetJsonField` _jsonobjectwrapper "Character Position" (`Actor.K2_GetActorLocation` (`GameplayStatics.GetPlayerPawn` 0)))
    (`|SetJsonField` _jsonobjectwrapper_2 "Data" (`|MakeArray` _jsonobjectwrapper_4 _jsonobjectwrapper_3 _jsonobjectwrapper_5 _jsonobjectwrapper))
    (`/Game/Telemetry/TelemetryService.Set Section` (`self.TelemetryService`) "Roaming")
    (`/Game/Telemetry/TelemetryService.Log Event` (`self.TelemetryService`) "Nav Move" "" _jsonobjectwrapper_2)))

(fn `LogPasscodeData`
  (params (`Event Name` :type String) (`Mouse Screen Position` :type "Vector2D Structure") (`Key Pressed` :type "Key Structure" :default "None"))
  (bind _jsonobjectwrapper (make `JsonObjectWrapper`))
  (bind _jsonobjectwrapper_2 (make `JsonObjectWrapper`))
  (bind _jsonobjectwrapper_3 (make `JsonObjectWrapper`))
  (bind _jsonobjectwrapper_4 (make `JsonObjectWrapper`))
  (if (`self.Success`)
    (`|SetJsonField` _jsonobjectwrapper_4 "Event ID" `Event Name`)
    (`|SetJsonField` _jsonobjectwrapper_3 "Mouse Screen Position" `Mouse Screen Position`)
    (`|SetJsonField` _jsonobjectwrapper "Key Pressed" `Key Pressed`)
    (`|SetJsonField` _jsonobjectwrapper_2 "Data" (`|MakeArray` _jsonobjectwrapper_4 _jsonobjectwrapper_3 _jsonobjectwrapper))
    (`/Game/Telemetry/TelemetryService.Set Section` (`self.TelemetryService`) "MiniGame")
    (`/Game/Telemetry/TelemetryService.Log Event` (`self.TelemetryService`) "PasscodeUI" "" _jsonobjectwrapper_2)))

(fn `LogPowerData`
  (params (`Event Name` :type String) (`Button Name` :type String) (ButtonSelected :type Boolean))
  (bind _jsonobjectwrapper (make `JsonObjectWrapper`))
  (bind _jsonobjectwrapper_2 (make `JsonObjectWrapper`))
  (bind _jsonobjectwrapper_3 (make `JsonObjectWrapper`))
  (bind _jsonobjectwrapper_4 (make `JsonObjectWrapper`))
  (bind _jsonobjectwrapper_5 (make `JsonObjectWrapper`))
  (bind (_locationx _locationy _returnvalue) (`PlayerController.GetMousePosition` (`GameplayStatics.GetPlayerController` 0)))
  (if (`self.Success`)
    (if _returnvalue
      (`|SetJsonField` _jsonobjectwrapper_2 "Event ID" (`KismetSystemLibrary.MakeLiteralString` `Event Name`))
      (`|SetJsonField` _jsonobjectwrapper_3 "Mouse Position" (`KismetMathLibrary.MakeVector2D` _locationx _locationy))
      (if true
        (`|SetJsonField` _jsonobjectwrapper_5 "Button Name" `Button Name`))
      (`|SetJsonField` _jsonobjectwrapper "Button Selected" ButtonSelected)
      (`|SetJsonField` _jsonobjectwrapper_4 "Data" (`|MakeArray` _jsonobjectwrapper_2 _jsonobjectwrapper_3 _jsonobjectwrapper_5 _jsonobjectwrapper))
      (`/Game/Telemetry/TelemetryService.Set Section` (`self.TelemetryService`) "MiniGame")
      (`/Game/Telemetry/TelemetryService.Log Event` (`self.TelemetryService`) "PowerGridUI" "" _jsonobjectwrapper_4))))

(fn `LogScannerData`
  (params (`Event Name` :type String) (MouseWorldPosition :type "Vector Structure"))
  (bind _jsonobjectwrapper (make `JsonObjectWrapper`))
  (bind _jsonobjectwrapper_2 (make `JsonObjectWrapper`))
  (bind _jsonobjectwrapper_3 (make `JsonObjectWrapper`))
  (if (`self.Success`)
    (`|SetJsonField` _jsonobjectwrapper_3 "Event ID" `Event Name`)
    (`|SetJsonField` _jsonobjectwrapper_2 "Mouse World Position" MouseWorldPosition)
    (`|SetJsonField` _jsonobjectwrapper "Data" (`|MakeArray` _jsonobjectwrapper_3 _jsonobjectwrapper_2))
    (`/Game/Telemetry/TelemetryService.Set Section` (`self.TelemetryService`) "MiniGame")
    (`/Game/Telemetry/TelemetryService.Log Event` (`self.TelemetryService`) "Scanner" "" _jsonobjectwrapper)))
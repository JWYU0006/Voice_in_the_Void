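; BP_Interaction detects and highlights objects tagged Interactable under the mouse cursor.
; Each tick it traces from the camera through the cursor, then runs a Visibility trace from the player pawn to reject wall-blocked objects.
; Accepted objects get a highlight material and are passed to BP_PlayerController as InteractableTarget with Highlighted set.
; Hitting an untagged actor restores the cached original material and clears Highlighted, but not InteractableTarget.
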(event `self.ReceiveTick`
  (params (DeltaSeconds :type "Float (single-precision)"))
  (bind (_locationx _locationy) (`PlayerController.GetMousePosition` (`GameplayStatics.GetPlayerController` 0)))
  (bind (_worldposition _worlddirection) (`GameplayStatics.DeprojectScreenToWorld` (`GameplayStatics.GetPlayerController` 0) (`KismetMathLibrary.MakeVector2D` _locationx _locationy)))
  ; Check if object detected is interactable
  (bind _outhit (`KismetSystemLibrary.LineTraceSingle` :`Start` (`PlayerCameraManager.GetCameraLocation` (`GameplayStatics.GetPlayerCameraManager` 0)) :`End` (+ _worldposition (* _worlddirection 10000)) :`TraceChannel` "TraceTypeQuery3" :`DrawDebugType` "ForOneFrame"))
  (if (`KismetSystemLibrary.IsValid` (`.HitActor` (`GameplayStatics.BreakHitResult` _outhit)))
    (if (`self.ActorHasTag` (`.HitActor` (`GameplayStatics.BreakHitResult` _outhit)) "Interactable")
      (if (not (== (`.HitActor` (`GameplayStatics.BreakHitResult` _outhit)) (`self.LastHit`)))
        ; Check if a wall blocks view from character to object
        (bind _outhit_2 (`KismetSystemLibrary.LineTraceSingle` (`self.K2_GetActorLocation` (`GameplayStatics.GetPlayerPawn` 0)) (`self.K2_GetActorLocation` (`.HitActor` (`GameplayStatics.BreakHitResult` _outhit))) "TraceTypeQuery1" false (`|MakeArray` (`.HitActor` (`GameplayStatics.BreakHitResult` _outhit))) "ForOneFrame"))
        (if (not (`GameplayStatics.BreakHitResult` _outhit_2))
          ; Highlight and select object for interaction
          (bind _asbp_player_controller (cast `/Game/_Data/Character/BP_PlayerController` (`GameplayStatics.GetPlayerController` 0)))
          (set `/Game/_Data/Character/BP_PlayerController.InteractableTarget` (`.HitActor` (`GameplayStatics.BreakHitResult` _outhit)) _asbp_player_controller)
          (set `self.LastHit` (`.HitActor` (`GameplayStatics.BreakHitResult` _outhit)))
          (set `self.OGMaterial` (`PrimitiveComponent.GetMaterial` (`self.GetComponentByClass` (`self.LastHit`) "/Script/Engine.StaticMeshComponent") 0))
          (`PrimitiveComponent.SetMaterial` (`.HitComponent` (`GameplayStatics.BreakHitResult` _outhit)) 0 "/Game/_Data/Material/Highlight.Highlight")
          (bind _asbp_player_controller_2 (cast `/Game/_Data/Character/BP_PlayerController` (`GameplayStatics.GetPlayerController` 0)))
          (set `/Game/_Data/Character/BP_PlayerController.Highlighted` true _asbp_player_controller_2)))
      (else
        ; Reset variables if object is no longer selected
        (if (`KismetSystemLibrary.IsValid` (`self.LastHit`))
          (`PrimitiveComponent.SetMaterial` (`self.GetComponentByClass` (`self.LastHit`) "/Script/Engine.StaticMeshComponent") 0 (`self.OGMaterial`))
          (set `self.LastHit` null)
          (set `self.OGMaterial` null)
          (bind _asbp_player_controller_3 (cast `/Game/_Data/Character/BP_PlayerController` (`GameplayStatics.GetPlayerController` 0)))
          (set `/Game/_Data/Character/BP_PlayerController.Highlighted` false _asbp_player_controller_3))))))

(fn `UserConstructionScript`)
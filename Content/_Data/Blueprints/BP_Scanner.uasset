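; Scanner spotlight that follows the player pawn while the controller's IsScanner flag is on and is parked far off otherwise.
; Each tick it aims at the hit of a camera trace toward ScreenToWorldPoint.
; It publishes origin and direction to MPC_Scanner for materials to read.
; While scanning, a Delay on Tick throttles logging of the hit position to GI_VoiceInTheVoid to about once a second.
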(event `self.ReceiveTick`
  (params (DeltaSeconds :type "Float (single-precision)"))
  (bind _asbp_player_controller (cast `/Game/_Data/Character/BP_PlayerController` (`GameplayStatics.GetPlayerController` 0)))
  (if (`/Game/_Data/Character/BP_PlayerController.IsScanner` _asbp_player_controller)
    (`SceneComponent.K2_SetWorldLocation` (`self.SpotLight`) (`self.K2_GetActorLocation` (`GameplayStatics.GetPlayerPawn` 0)) false false)
    (else
      (`SceneComponent.K2_SetWorldLocation` (`self.SpotLight`) (-10000.0 0.0 0.0) false false)))
  (bind _outhit (`KismetSystemLibrary.LineTraceSingle` :`Start` (`PlayerCameraManager.GetCameraLocation` (`GameplayStatics.GetPlayerCameraManager` 0)) :`End` (`self.ScreenToWorldPoint`) :`TraceChannel` "TraceTypeQuery1" :`DrawDebugType` "ForOneFrame"))
  (`SceneComponent.K2_SetWorldRotation` (`self.SpotLight`) (`KismetMathLibrary.FindLookAtRotation` (`SceneComponent.K2_GetComponentLocation` (`self.SpotLight`)) (`.Location` (`GameplayStatics.BreakHitResult` _outhit))) false false)
  (`KismetMaterialLibrary.SetVectorParameterValue` "/Game/_Data/Material/MPC_Scanner.MPC_Scanner" "ScannerOrigin" (`KismetMathLibrary.Conv_VectorToLinearColor` (`SceneComponent.K2_GetComponentLocation` (`self.SpotLight`))))
  (`KismetMaterialLibrary.SetVectorParameterValue` "/Game/_Data/Material/MPC_Scanner.MPC_Scanner" "ScannerDirection" (`KismetMathLibrary.Conv_VectorToLinearColor` (`SceneComponent.GetForwardVector` (`self.SpotLight`))))
  (bind _asbp_player_controller_2 (cast `/Game/_Data/Character/BP_PlayerController` (`GameplayStatics.GetPlayerController` 0)))
  (if (`/Game/_Data/Character/BP_PlayerController.IsScanner` _asbp_player_controller_2)
    (bind _asgi_voice_in_the_void (cast `/Game/_Data/Blueprints/GI_VoiceInTheVoid` (`GameplayStatics.GetGameInstance`)))
    (`KismetSystemLibrary.Delay` 1.0)
    (`/Game/_Data/Blueprints/GI_VoiceInTheVoid.LogScannerData` _asgi_voice_in_the_void "Scanning" (`.Location` (`GameplayStatics.BreakHitResult` _outhit)))))

(fn `UserConstructionScript`)
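; BP_FixedCamera is a fixed-position camera actor that becomes the player's view through a blended view-target switch whenever an overlap begins on it.
; Each tick it projects the player pawn to screen space and checks whether it nears the left or right viewport edge within a set margin.
; When it does, RotateCameraToPawn eases only the camera's yaw toward the pawn, keeping pitch and zeroing roll.
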(event `self.ReceiveActorBeginOverlap`
  (params (OtherActor :type "Actor Object Reference"))
  ; Set camera if collision occurs
  (`PlayerController.SetViewTargetWithBlend` (`GameplayStatics.GetPlayerController` 0) (`ActorComponent.GetOwner` (`self.Camera`)) 0.0 "VTBlend_Linear" 0.0 false))

(event `self.ReceiveTick`
  (params (DeltaSeconds :type "Float (single-precision)"))
  (bind _returnvalue_x (`KismetMathLibrary.BreakVector2D` (`WidgetLayoutLibrary.GetViewportSize`)))
  (bind _distancefromscreen (`self.distanceFromScreen`))
  (bind _screenposition (`GameplayStatics.ProjectWorldToScreen` (`GameplayStatics.GetPlayerController` 0) (`self.K2_GetActorLocation` (`GameplayStatics.GetPlayerPawn` 0))))
  (if (or (> (`KismetMathLibrary.BreakVector2D` _screenposition) (- _returnvalue_x _distancefromscreen)) (< (`KismetMathLibrary.BreakVector2D` _screenposition) _distancefromscreen))
    (`self.RotateCameraToPawn` DeltaSeconds)))

(fn `RotateCameraToPawn`
  (params (DeltaTime :type "Float (single-precision)"))
  (locals (NewLocalVar :type "Rotator Structure" :default (struct)))
  (bind (_returnvalue_roll _returnvalue_pitch) (`KismetMathLibrary.BreakRotator` (`SceneComponent.K2_GetComponentRotation` (`self.Camera`))))
  (bind (_returnvalue_roll_2 _returnvalue_pitch_2 _returnvalue_yaw) (`KismetMathLibrary.BreakRotator` (`KismetMathLibrary.RInterpTo` (`SceneComponent.K2_GetComponentRotation` (`self.Camera`)) (`KismetMathLibrary.FindLookAtRotation` (`SceneComponent.K2_GetComponentLocation` (`self.Camera`)) (`self.K2_GetActorLocation` (`GameplayStatics.GetPlayerPawn` 0))) DeltaTime (`self.camRotSpd`))))
  (`SceneComponent.K2_SetWorldRotation` (`self.Camera`) (`KismetMathLibrary.MakeRotator` 0.0 _returnvalue_pitch _returnvalue_yaw) false false))

(fn `UserConstructionScript`)